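; BP_Player is the player character Blueprint, handling the health HUD, a roll and melee combat input.
; It creates WBP_PlayerHUD on begin play and refreshes its health whenever damage is taken.
; Toggling combat mode plays draw or sheathe montages, then re-attaches the weapon after a fixed delay.
; Fast and heavy attacks share DoAttack, which instantly arms the weapon if needed and blocks overlapping attack or roll montages.
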(event `self.ReceiveBeginPlay`
  ;[1 1 1] Brgin Play
  (bind _returnvalue (`|CreateWidget` "/Game/Widgets/WBP_PlayerHUD.WBP_PlayerHUD_C"))
  (bind _output_get (set `self.PlayerHUD` _returnvalue))
  (`UserWidget.AddToViewport` _output_get 0))

(event `InputAction|Roll`
  (params (Key :type "Key Structure"))
  ;[1 1 1] Кувырок (Супер сырой)
  (:`Pressed`
    (`self.Roll` "/Game/Characters/Admin/Animation/Locomotion/AM_Locomotion_Roll.AM_Locomotion_Roll" 1.5 "Roll")))

(event `self.ReceiveAnyDamage`
  (params (Damage :type "Float (single-precision)") (DamageType :type "DamageType Object Reference") (InstigatedBy :type "Controller Object Reference") (DamageCauser :type "Actor Object Reference"))
  (bind _health (`self.Health`))
  ;[1 1 1] HP Widget Update
  (`/Engine/EditorBlueprintResources/StandardMacros.IsValid` (`self.PlayerHUD`)
    (:`Is Valid`
      (`/Game/Widgets/WBP_PlayerHUD.UpdateHealth` (`self.PlayerHUD`) (`HealthComponent.Health` _health) (`HealthComponent.DefaultHealth` _health)))))

(event `InputAction|AttackFast`
  (params (Key :type "Key Structure"))
  ;[1 1 1] Лёгкая атака
  (:`Pressed`
    (`self.DoAttack` "/Game/Characters/Admin/Animation/Weapon/AM_Weapon.AM_Weapon" 1.3 0.0 "FastAttack")))

(event `InputAction|AttackStrong`
  (params (Key :type "Key Structure"))
  ;[1 1 1] Сильная атака
  (:`Pressed`
    (`self.DoAttack` "/Game/Characters/Admin/Animation/Weapon/AM_Weapon.AM_Weapon" 1.0 0.0 "HeavyAttack")))

(event `InputAction|CombatMode`
  (params (Key :type "Key Structure"))
  ;[1 1 1] Достать/Убрать оружие
  (:`Pressed`
    (`self.SetCombatMode`)))

(event `self.SetCombatMode`
  ;[1 1 1] Достать/Убрать оружие
  (if (`KismetSystemLibrary.IsValid` (`self.MeleeWeapon`))
    (if (not (`AnimInstance.IsAnyMontagePlaying` (`SkeletalMeshComponent.GetAnimInstance` (`self.Mesh`))))
      (set `self.bCombatMode` (not (`self.bCombatMode`)))
      (if (`self.bCombatMode`)
        (`|PlayMontage` (`self.Mesh`) "/Game/Characters/Admin/Animation/Weapon/AM_Weapon.AM_Weapon" 1.3 0.0 "DrawWeapon"
          (:`then`
            (`KismetSystemLibrary.Delay` 0.8)
            (`self.K2_AttachToComponent` (`self.MeleeWeapon`) (`self.MeleeWeaponArmed`) "None" "SnapToTarget" "SnapToTarget" "KeepRelative" true)))
        (else
          (`|PlayMontage` (`self.Mesh`) "/Game/Characters/Admin/Animation/Weapon/AM_Weapon.AM_Weapon" 1.3 0.0 "SeathWeapon"
            (:`then`
              (`KismetSystemLibrary.Delay` 0.8)
              (`self.K2_AttachToComponent` (`self.MeleeWeapon`) (`self.MeleeWeaponUnarmed`) "None" "SnapToTarget" "SnapToTarget" "KeepRelative" true))))))))

(event `DoAttack`
  (params (MontageToPlay :type "AnimMontage Object Reference") (PlayRate :type "Float (double-precision)") (StartingPosition :type "Float (double-precision)") (StartingSection :type Name))
  (bind _returnvalue (`SkeletalMeshComponent.GetAnimInstance` (`self.Mesh`)))
  ;[1 1 1] Атаковать
  (if (`KismetSystemLibrary.IsValid` (`self.MeleeWeapon`))
    (if (not (`self.bCombatMode`))
      (set `self.bCombatMode` (not (`self.bCombatMode`)))
      (`self.K2_AttachToComponent` (`self.MeleeWeapon`) (`self.MeleeWeaponArmed`) "None" "SnapToTarget" "SnapToTarget" "KeepRelative" true))
    (if (not (or (`AnimInstance.Montage_IsPlaying` _returnvalue "/Game/Characters/Admin/Animation/Weapon/AM_Weapon.AM_Weapon") (`AnimInstance.Montage_IsPlaying` _returnvalue "/Game/Characters/Admin/Animation/Locomotion/AM_Locomotion_Roll.AM_Locomotion_Roll")))
      (`|PlayMontage` (`self.Mesh`) MontageToPlay PlayRate StartingPosition StartingSection))))

(fn `UserConstructionScript`)