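; BP_ZombieController is the AI controller for zombies, driving them through the BT_Zombie behavior tree.
; On possession it runs the tree and stores the possessed pawn in the blackboard as SelfActor.
; AI Perception updates involving BP_Player set TargetActor and mirror the sensing result into bPlayerCanBeSeen.
; TargetActor stays set when sensing fails, as only the boolean reflects the loss.
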(event `self.ReceivePossess`
  (params (PossessedPawn :type "Pawn Object Reference"))
  ;[1 1 1] On Possess
  (`self.RunBehaviorTree` "/Game/Characters/Enemies/AI/BT_Zombie.BT_Zombie")
  (`BlackboardComponent.SetValueAsObject` (`AIBlueprintHelperLibrary.GetBlackboard` null) "SelfActor" PossessedPawn))

(event `self.AIPerception.OnTargetPerceptionUpdated`
  (params (Actor :type "Actor Object Reference") (Stimulus :type "AIStimulus Structure"))
  (bind _returnvalue (`AIBlueprintHelperLibrary.GetBlackboard` null))
  ;[1 1 1] Если кого-то видно
  (bind _asbp_player (cast `/Game/Characters/Admin/Blueprints/BP_Player` Actor))
  (`BlackboardComponent.SetValueAsObject` _returnvalue "TargetActor" _asbp_player)
  (`BlackboardComponent.SetValueAsBool` _returnvalue "bPlayerCanBeSeen" (`.bSuccessfullySensed` (break `AIStimulus` Stimulus))))

(fn `UserConstructionScript`)