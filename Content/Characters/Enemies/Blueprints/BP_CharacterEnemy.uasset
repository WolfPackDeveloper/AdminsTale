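; Enemy character Blueprint that shows health and damage feedback and handles hit reactions and melee combat stance.
; BeginPlay and AnyDamage refresh a health bar widget from the Health component, with damage also shown as battle text.
; Hit reactions and stance switches skip any active montage section to its end before playing theirs; stance switches reattach the weapon between armed and unarmed components after a delay.
; DoAttack is empty, and leftover attack logic is disconnected.
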(event `self.ReceiveBeginPlay`
  ;[1 1 1] BeginPlay
  (`self.UpdateHealthBar`))

(event `self.ReceiveAnyDamage`
  (params (Damage :type "Float (single-precision)") (DamageType :type "DamageType Object Reference") (InstigatedBy :type "Controller Object Reference") (DamageCauser :type "Actor Object Reference"))
  ;[1 1 1] Получение урона
  (`self.UpdateHealthBar`)
  (`self.Display Damage` Damage))

(event `DoAttack`
  (params (DamageMultiplier :type "Float (double-precision)") (MontageToPlay :type "AnimMontage Object Reference") (PlayRate :type "Float (double-precision)") (StartingSection :type Name))
  ;[1 1 1] Атаковать
)

(event `UpdateHealthBar`
  (bind _health (`self.Health`))
  ;[1 1 1] Получение урона
  (bind _aswbp_ai_healthbar (cast `/Game/Widgets/AI/WBP_AI_Healthbar` (`WidgetComponent.GetUserWidgetObject` (`self.HealthBar`))))
  (`/Engine/EditorBlueprintResources/StandardMacros.IsValid` _aswbp_ai_healthbar
    (:`Is Valid`
      (`/Game/Widgets/AI/WBP_AI_Healthbar.UpdateHealth` _aswbp_ai_healthbar (`HealthComponent.Health` _health) (`HealthComponent.MaxHealth` _health)))))

(event `Display Damage`
  (params (Damage :type "Float (double-precision)"))
  ;[1 1 1] Получение урона
  (bind _aswbp_ai_battle_text (cast `/Game/Widgets/AI/WBP_AI_BattleText` (`WidgetComponent.GetUserWidgetObject` (`self.BattleText`))))
  (`/Engine/EditorBlueprintResources/StandardMacros.IsValid` _aswbp_ai_battle_text
    (:`Is Valid`
      (`/Game/Widgets/AI/WBP_AI_BattleText.DisplayDamage` _aswbp_ai_battle_text Damage))))

(event `GetHitReaction`
  (params (AnimMontage :type "AnimMontage Object Reference") (InPlayRate :type "Float (double-precision)") (StartSectionName :type Name))
  (bind _returnvalue (`SkeletalMeshComponent.GetAnimInstance` (`self.Mesh`)))
  (bind _returnvalue_2 (`AnimInstance.GetCurrentActiveMontage` _returnvalue))
  ;[1 1 1] Получение урона
  (if (`AnimInstance.IsAnyMontagePlaying` _returnvalue)
    (`AnimInstance.Montage_JumpToSectionsEnd` _returnvalue (`AnimInstance.Montage_GetCurrentSection` _returnvalue _returnvalue_2) _returnvalue_2))
  (`self.PlayAnimMontage` AnimMontage InPlayRate StartSectionName))

(event `SwitchCombatMode`
  (params (bCombatMode :type Boolean) (MontageToPlay :type "AnimMontage Object Reference") (PlayRate :type "Float (double-precision)") (StartingSection :type Name))
  (bind _returnvalue (`SkeletalMeshComponent.GetAnimInstance` (`self.Mesh`)))
  (bind _returnvalue_2 (`AnimInstance.GetCurrentActiveMontage` _returnvalue))
  ;[1 1 1] Переход в боевой режим и обратно
  (`/Engine/EditorBlueprintResources/StandardMacros.IsValid` (`self.MeleeWeapon`)
    (:`Is Valid`
      (if (`AnimInstance.IsAnyMontagePlaying` _returnvalue)
        (`AnimInstance.Montage_JumpToSectionsEnd` _returnvalue (`AnimInstance.Montage_GetCurrentSection` _returnvalue _returnvalue_2) _returnvalue_2))
      (set `self.bCombatMode` bCombatMode)
      (`self.PlayAnimMontage` MontageToPlay PlayRate StartingSection)
      (`KismetSystemLibrary.Delay` 0.8)
      (if (`self.bCombatMode`)
        (`self.K2_AttachToComponent` (`self.MeleeWeapon`) (`self.MeleeWeaponArmed`) "None" "SnapToTarget" "SnapToTarget" "KeepRelative" true)
        (else
          (`self.K2_AttachToComponent` (`self.MeleeWeapon`) (`self.MeleeWeaponUnarmed`) "None" "SnapToTarget" "SnapToTarget" "KeepRelative" true))))))

(fn `UserConstructionScript`)